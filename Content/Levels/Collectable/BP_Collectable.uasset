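; BP_Collectable is a pickup actor that awards points to the player and can contribute to winning the game.
; When anything begins overlapping its Collision, it plays a sound and adds Cost to the score component of player 0's character.
; It then pushes the truncated score to the HUD, has GM_Game check for a win, and destroys itself.
; The overlapping actor is never checked.
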(event OnComponentBeginOverlap(Collision)
  (params (OverlappedComponent :type Primitive%20Component%20Object%20Reference) (OtherActor :type Actor%20Object%20Reference) (OtherComp :type Primitive%20Component%20Object%20Reference) (OtherBodyIndex :type Integer) (bFromSweep :type Boolean) (SweepResult :type Hit%20Result%20Structure%20%28by%20ref%29))
  (Audio|PlaySound2D (Variables|Default|GetSound) 1.0 1.0 0.0 0 0)
  (bind _asbp_third_person_character (Utilities|Casting|CastToBP_ThirdPersonCharacter (Game|GetPlayerCharacter 0)))
  (bind _output_get (Variables|/Game/Player/Score/BP_Score_AC.BP_Score_AC_C|SetScore (Variables|/Game/Player/ThirdPerson/Blueprints/BP_ThirdPersonCharacter.BP_ThirdPersonCharacter_C|GetBP_Score_AC _asbp_third_person_character) (+ (Variables|/Game/Player/Score/BP_Score_AC.BP_Score_AC_C|GetScore (Variables|/Game/Player/ThirdPerson/Blueprints/BP_ThirdPersonCharacter.BP_ThirdPersonCharacter_C|GetBP_Score_AC _asbp_third_person_character)) (Variables|Default|GetCost))))
  (bind _ashud_third_person (Utilities|Casting|CastToHUD_ThirdPerson (HUD|GetHUD (Game|GetPlayerController 0))))
  (Default|ScoreUpdate (Variables|/Game/Player/UI/HUD_ThirdPerson.HUD_ThirdPerson_C|GetHUD _ashud_third_person) (Math|Float|Truncate _output_get))
  (bind _asgm_game (Utilities|Casting|CastToGM_Game (Game|GetGameMode)))
  (Default|CheckWin _asgm_game)
  (Actor|DestroyActor))

(fn ConstructionScript)