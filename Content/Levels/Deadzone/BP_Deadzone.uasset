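; BP_Deadzone is a level hazard volume that sends the hero back on collision overlap.
; The overlap shows a widget, plays a sound and moves player 0's BP_Hero to the checkpoint stored in its BPProgressAC component.
; Without a valid checkpoint, the hero moves to the PlayerStart and input is disabled for the Disability delay.
; The overlapping actor is never checked, so any overlap triggers this response.
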(event OnComponentBeginOverlap(Collision)
  (params (OverlappedComponent :type Primitive%20Component%20Object%20Reference) (OtherActor :type Actor%20Object%20Reference) (OtherComp :type Primitive%20Component%20Object%20Reference) (OtherBodyIndex :type Integer) (bFromSweep :type Boolean) (SweepResult :type Hit%20Result%20Structure%20%28by%20ref%29))
  (bind _returnvalue (UserInterface|CreateWidget (Variables|Default|GetWidget) (Game|GetPlayerController 0)))
  (UserInterface|Viewport|AddtoViewport _returnvalue 0)
  (Audio|PlaySound2D (Variables|Default|GetSound) 1.0 1.0 0.0 0 0)
  (bind _asbp_hero (Utilities|Casting|CastToBP_Hero (Game|GetPlayerCharacter 0)))
  (Utilities|IsValid (Variables|/Game/Player/Progress/BP_Progress_AC.BP_Progress_AC_C|GetCheckpoint (Variables|/Game/Player/Character/Blueprints/BP_Hero.BP_Hero_C|GetBP_Progress_AC _asbp_hero))
    (:Is%20Valid
      (Transformation|SetActorLocation _asbp_hero (Transformation|GetActorLocation (Variables|/Game/Player/Progress/BP_Progress_AC.BP_Progress_AC_C|GetCheckpoint (Variables|/Game/Player/Character/Blueprints/BP_Hero.BP_Hero_C|GetBP_Progress_AC _asbp_hero))) false false))
    (:Is%20Not%20Valid
      (bind _returnvalue_2 (Actor|GetActorOfClass "/Script/Engine.PlayerStart"))
      (Transformation|SetActorLocation _asbp_hero (Transformation|GetActorLocation _returnvalue_2) false false)
      (Input|DisableInput (Game|GetPlayerCharacter 0) (Game|GetPlayerController 0))
      (Utilities|FlowControl|Delay (Variables|Default|GetDisability))
      (Input|EnableInput (Game|GetPlayerCharacter 0) (Game|GetPlayerController 0)))))

(fn ConstructionScript)