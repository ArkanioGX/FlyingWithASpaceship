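; Spike hazard actor that repeatedly raises and retracts its Spikes component on a timed cycle, starting raised at BeginPlay.
; TurnOn and TurnOff quickly move the component between its relative origin and a lowered position, each scheduling the other with a function-name timer.
; TimeOff sets the delay before retracting and TimeOn the delay before raising; the Blueprint contains no overlap or damage logic.
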(event Custom|TurnOn
  (Utilities|Time|SetTimerbyFunctionName 0 "TurnOff" (Variables|Default|GetTimeOff))
  (Components|MoveComponentTo (Variables|Default|Getspikes) "0, 0, 0" "0.000000,0.000000,90.000000" false false 0.06 false))

(event Custom|TurnOff
  (Utilities|Time|SetTimerbyFunctionName 0 "TurnOn" (Variables|Default|GetTimeOn))
  (Components|MoveComponentTo (Variables|Default|Getspikes) "0.000000,0.000000,-200.000000" "0.000000,0.000000,90.000000" false false 0.06 false))

(event EventBeginPlay
  (CallFunction|Turnon))

(event Collision|EventActorBeginOverlap
  (params (OtherActor :type Actor%20Object%20Reference)))

(event EventTick
  (params (DeltaSeconds :type Float%20%28single-precision%29)))

(fn ConstructionScript)