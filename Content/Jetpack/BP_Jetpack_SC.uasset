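; BP_Jetpack_SC is a jetpack Blueprint that lets the player's third-person character fly upward.
; On BeginPlay it caches player 0's BP_ThirdPersonCharacter.
; While IA_Fly triggers, it sets the character movement mode to Flying and applies upward movement input scaled by Force.
; When IA_Fly completes, it switches the mode to Falling.
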(event Input|EnhancedActionEvents|EnhancedInputActionIA_Fly
  (params (ActionValue :type Boolean) (ElapsedSeconds :type Float%20%28double-precision%29) (TriggeredSeconds :type Float%20%28double-precision%29) (InputAction :type Input%20Action%20Object%20Reference :default "/Game/Jetpack/InputActions/IA_Fly.IA_Fly"))
  (:Triggered
    (Pawn|Components|CharacterMovement|SetMovementMode (Variables|/Script/Engine.Character|GetCharacterMovement (Variables|Default|GetCharacter)) "MOVE_Flying" 0)
    (Pawn|Input|AddMovementInput (Variables|Default|GetCharacter) "0.000000,0.000000,1.000000" (Variables|Default|GetForce) false))
  (:Completed
    (Pawn|Components|CharacterMovement|SetMovementMode (Variables|/Script/Engine.Character|GetCharacterMovement (Variables|Default|GetCharacter)) "MOVE_Falling" 0)))

(event EventBeginPlay
  (bind _asbp_third_person_character (Utilities|Casting|CastToBP_ThirdPersonCharacter (Game|GetPlayerCharacter 0)))
  (Variables|Default|SetCharacter _asbp_third_person_character))