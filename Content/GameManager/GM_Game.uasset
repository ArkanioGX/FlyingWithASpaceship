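; Game manager Blueprint that handles the win condition for collecting BP_Collectable items.
; CheckWin counts the BP_Collectable actors in the level and treats exactly one remaining as a win, rather than zero.
; On a win it calls YouWin on HUD_Hero, shows the mouse cursor and switches the first player controller to Game and UI input.
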(event Custom|CheckWin
  (bind _returnvalue (Game|GetPlayerController 0))
  (bind _outactors (Actor|GetAllActorsOfClass "/Game/GameManager/GPE/BP_Collectable.BP_Collectable_C"))
  (if (== (Utilities|Array|Length _outactors) 1)
    (bind _ashud_hero (Utilities|Casting|CastToHUD_Hero (HUD|GetHUD (Game|GetPlayerController 0))))
    (Default|YouWin _ashud_hero)
    (Variables|/Script/Engine.PlayerController|SetbShowMouseCursor _returnvalue true)
    (Input|SetInputModeGameandUI _returnvalue 0 "DoNotLock" true false)))

(fn ConstructionScript)