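; BP_CoinDoor is a door that removes itself once the player has collected enough coins.
; A text render shows the Score from PC_Hero against CoinsNeeded, set on BeginPlay and refreshed on each CheckScore.
; CheckScore destroys the actor when the truncated score reaches that threshold, while OpenDoor destroys it unconditionally.
; Nothing in this graph calls either event, and Tick and overlap are unused.
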(event Custom|CheckScore
  (bind _aspc_hero (Utilities|Casting|CastToPC_Hero (Game|GetPlayerController 0)))
  (CallFunction|UpdateText)
  (if (>= (Math|Float|Truncate (Variables|/Game/GameManager/Player/BP_Score_AC.BP_Score_AC_C|GetScore (Variables|/Game/GameManager/Player/PC_Hero.PC_Hero_C|GetScore _aspc_hero))) (Variables|Default|GetCoinsNeeded))
    (Actor|DestroyActor)))

(event Custom|OpenDoor
  (Actor|DestroyActor))

(event Custom|Update%20Text
  (bind _aspc_hero (Utilities|Casting|CastToPC_Hero (Game|GetPlayerController 0)))
  (Rendering|Components|TextRender|SetText (Variables|Default|GetTextRender) (Utilities|Text|ToText(String) (Utilities|String|Append "Coins Needed : " (Utilities|String|ToString(Integer) (Math|Float|Truncate (Variables|/Game/GameManager/Player/BP_Score_AC.BP_Score_AC_C|GetScore (Variables|/Game/GameManager/Player/PC_Hero.PC_Hero_C|GetScore _aspc_hero)))) " / " (Utilities|String|ToString(Integer) (Variables|Default|GetCoinsNeeded))))))

(event EventBeginPlay
  (CallFunction|UpdateText))

(event Collision|EventActorBeginOverlap
  (params (OtherActor :type Actor%20Object%20Reference)))

(event EventTick
  (params (DeltaSeconds :type Float%20%28single-precision%29)))

(fn ConstructionScript)