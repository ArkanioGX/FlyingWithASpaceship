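; BP_Breakable is an obstacle that a boosting spaceship can smash for points.
; When BP_Spaceship overlaps its Trigger while boosting, it adds the breakable reward from Data to the score held by PC_Hero.
; It then pushes the truncated score to the HUD through HUD_Hero and destroys itself.
; Overlaps by other actors or a non-boosting ship do nothing.
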(event OnComponentBeginOverlap(Trigger)
  (params (OverlappedComponent :type Primitive%20Component%20Object%20Reference) (OtherActor :type Actor%20Object%20Reference) (OtherComp :type Primitive%20Component%20Object%20Reference) (OtherBodyIndex :type Integer) (bFromSweep :type Boolean) (SweepResult :type Hit%20Result%20Structure%20%28by%20ref%29))
  (bind _asbp_spaceship (Utilities|Casting|CastToBP_Spaceship OtherActor))
  (if (Variables|/Game/GameManager/Player/BP_Spaceship.BP_Spaceship_C|GetisBoosting _asbp_spaceship)
    (Variables|/Game/GameManager/Player/BP_Score_AC.BP_Score_AC_C|SetScore (Variables|/Game/GameManager/Player/PC_Hero.PC_Hero_C|GetScore (.AsPC%20Hero (Utilities|Casting|CastToPC_Hero (Game|GetPlayerController 0)))) (+ (Variables|/Game/GameManager/Player/BP_Score_AC.BP_Score_AC_C|GetScore (Variables|/Game/GameManager/Player/PC_Hero.PC_Hero_C|GetScore (.AsPC%20Hero (Utilities|Casting|CastToPC_Hero (Game|GetPlayerController 0))))) (Variables|/Game/GameManager/Player/DR_SpaceShip.DR_SpaceShip_C|GetBreakableRewardGiven (Variables|Default|GetData))))
    (Default|ScoreUpdate (Variables|/Game/GameManager/UI/HUD_Hero.HUD_Hero_C|GetHUD (.AsHUD%20Hero (Utilities|Casting|CastToHUD_Hero (HUD|GetHUD (Game|GetPlayerController 0))))) (Math|Float|Truncate (Variables|/Game/GameManager/Player/BP_Score_AC.BP_Score_AC_C|GetScore (Variables|/Game/GameManager/Player/PC_Hero.PC_Hero_C|GetScore (.AsPC%20Hero (Utilities|Casting|CastToPC_Hero (Game|GetPlayerController 0)))))))
    (Actor|DestroyActor)))

(fn ConstructionScript)