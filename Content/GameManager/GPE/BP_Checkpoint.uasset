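; Checkpoint actor that saves a respawn point for the player hero and signals it with effects.
; An overlap on Collision writes the Respawn component's world location to Checkpoint in the hero's BPProgressAC component.
; A Niagara burst above the actor and a 2D sound play only when that location differs from the stored one.
; The overlap always targets player character 0, without checking which actor entered.
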(event OnComponentBeginOverlap(Collision)
  (params (OverlappedComponent :type Primitive%20Component%20Object%20Reference) (OtherActor :type Actor%20Object%20Reference) (OtherComp :type Primitive%20Component%20Object%20Reference) (OtherBodyIndex :type Integer) (bFromSweep :type Boolean) (SweepResult :type Hit%20Result%20Structure%20%28by%20ref%29))
  (bind _asbp_hero (Utilities|Casting|CastToBP_Hero (Game|GetPlayerCharacter 0)))
  (if (not (Utilities|Operators|EqualEqual (Variables|/Game/GameManager/Player/BP_Progress_AC.BP_Progress_AC_C|GetCheckpoint (Variables|/Game/GameManager/Player/BP_Hero.BP_Hero_C|GetBP_Progress_AC _asbp_hero)) (Transformation|GetWorldLocation (Variables|Default|GetRespawn)) 0.1))
    (Variables|/Game/GameManager/Player/BP_Progress_AC.BP_Progress_AC_C|SetCheckpoint (Variables|/Game/GameManager/Player/BP_Hero.BP_Hero_C|GetBP_Progress_AC _asbp_hero) (Transformation|GetWorldLocation (Variables|Default|GetRespawn)))
    (Niagara|SpawnSystematLocation (Variables|Default|GetNiagara) (+ (Transformation|GetActorLocation) "0.000000,0.000000,200.000000"))
    (Audio|PlaySound2D (Variables|Default|GetSound) 1.0 1.0 0.0 0 0)))

(fn ConstructionScript)