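; BP_Deadzone is a trigger volume that kills the player's BP_Hero on overlap and respawns it.
; A DoOnce-guarded sequence flags death, sets falling movement, disables input, plays a sound and death montage, and shows a widget after a short delay.
; On montage completion, it moves the hero to the progress component's checkpoint, or PlayerStart if that component is invalid.
; After a delay, it removes the widget, restores input, calls Respawn and re-arms.
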(event OnComponentBeginOverlap(Trigger)
  (params (OverlappedComponent :type Primitive%20Component%20Object%20Reference) (OtherActor :type Actor%20Object%20Reference) (OtherComp :type Primitive%20Component%20Object%20Reference) (OtherBodyIndex :type Integer) (bFromSweep :type Boolean) (SweepResult :type Hit%20Result%20Structure%20%28by%20ref%29))
  (bind _returnvalue (Game|GetPlayerCharacter 0))
  (bind _asbp_hero (Utilities|Casting|CastToBP_Hero _returnvalue))
  (if (== OtherActor (Game|GetPlayerCharacter 0))
    (Utilities|FlowControl|DoOnce false :!label _label
      (:Completed
        (Variables|/Game/GameManager/Player/BP_Hero.BP_Hero_C|SetisDead _asbp_hero true)
        (Pawn|Components|CharacterMovement|SetMovementMode (Variables|/Script/Engine.Character|GetCharacterMovement _asbp_hero) "MOVE_Falling" 0)
        (Input|DisableInput (Game|GetPlayerCharacter 0) (Game|GetPlayerController 0))
        (Audio|PlaySound2D (Variables|Default|GetSound) 1.0 1.0 0.0 0 0)
        (Animation|Montage|PlayMontage (Variables|/Script/Engine.Character|GetMesh (.AsBP%20Hero (Utilities|Casting|CastToBP_Hero (Game|GetPlayerCharacter 0)))) "/Game/Assets/Animations/AM_Death.AM_Death" 1.0 0.0 "Default"
          (:then
            (Utilities|FlowControl|Delay 0.5)
            (bind _returnvalue_2 (UserInterface|CreateWidget (Variables|Default|GetWidgetToCreate) (Game|GetPlayerController 0)))
            (Variables|Default|SetWidget _returnvalue_2)
            (UserInterface|Viewport|AddtoViewport (Variables|Default|GetWidget) 0))
          (:OnCompleted
            (bind _asbp_hero_2 (Utilities|Casting|CastToBP_Hero (Game|GetPlayerCharacter 0)))
            (Utilities|IsValid (Variables|/Game/GameManager/Player/BP_Hero.BP_Hero_C|GetBP_Progress_AC _asbp_hero_2)
              (:Is%20Valid
                (Transformation|SetActorLocation _asbp_hero_2 (Variables|/Game/GameManager/GPE/BP_Checkpoint.BP_Checkpoint_C|Getrespawn%20location (Variables|/Game/GameManager/Player/BP_Progress_AC.BP_Progress_AC_C|GetCheckpoint (Variables|/Game/GameManager/Player/BP_Hero.BP_Hero_C|GetBP_Progress_AC _asbp_hero_2))) false false))
              (:Is%20Not%20Valid
                (bind _returnvalue_3 (Actor|GetActorOfClass "/Script/Engine.PlayerStart"))
                (Transformation|SetActorLocation _asbp_hero_2 (Transformation|GetActorLocation _returnvalue_3) false false)))
            (Utilities|FlowControl|Delay (Variables|Default|GetDisability))
            (Widget|RemovefromParent (Variables|Default|GetWidget))
            (Input|EnableInput (Game|GetPlayerCharacter 0) (Game|GetPlayerController 0))
            (Default|Respawn (.AsBP%20Hero (Utilities|Casting|CastToBP_Hero (Game|GetPlayerCharacter 0))))
            (goto _label Reset)))))))

(fn ConstructionScript)