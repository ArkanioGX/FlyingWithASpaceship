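; BP_Collectable is a pickup actor that awards score when the player pawn overlaps its trigger.
; On overlap it plays a sound, adds its Cost to the PC_Hero controller's score, and refreshes the HUD_Hero widget with a coin-collect animation.
; It then asks GM_Game to check the win condition, spawns a Niagara effect at its location and destroys itself.
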(event OnComponentBeginOverlap(Trigger)
  (params (OverlappedComponent :type Primitive%20Component%20Object%20Reference) (OtherActor :type Actor%20Object%20Reference) (OtherComp :type Primitive%20Component%20Object%20Reference) (OtherBodyIndex :type Integer) (bFromSweep :type Boolean) (SweepResult :type Hit%20Result%20Structure%20%28by%20ref%29))
  ;[0 0 0 1 16] Check if it is player
  (if (== OtherActor (Game|Player|GetPlayerPawn 0))
    (Audio|PlaySound2D (Variables|Default|GetSound) 1.0 1.0 0.0 0 0)
    (bind _output_get (Variables|/Game/GameManager/Player/BP_Score_AC.BP_Score_AC_C|SetScore (Variables|/Game/GameManager/Player/PC_Hero.PC_Hero_C|GetScore (.AsPC%20Hero (Utilities|Casting|CastToPC_Hero (Game|GetPlayerController 0)))) (+ (Variables|/Game/GameManager/Player/BP_Score_AC.BP_Score_AC_C|GetScore (Variables|/Game/GameManager/Player/PC_Hero.PC_Hero_C|GetScore (.AsPC%20Hero (Utilities|Casting|CastToPC_Hero (Game|GetPlayerController 0))))) (Variables|Default|GetCost))))
    (Default|ScoreUpdate (Variables|/Game/GameManager/UI/HUD_Hero.HUD_Hero_C|GetHUD (.AsHUD%20Hero (Utilities|Casting|CastToHUD_Hero (HUD|GetHUD (Game|GetPlayerController 0))))) (Math|Float|Truncate _output_get))
    (UserInterface|Animation|PlayAnimation (Variables|/Game/GameManager/UI/HUD_Hero.HUD_Hero_C|GetHUD (.AsHUD%20Hero (Utilities|Casting|CastToHUD_Hero (HUD|GetHUD (Game|GetPlayerController 0))))) (Variables|/Game/GameManager/UI/W_GameUI.W_GameUI_C|Getcoincollect (Variables|/Game/GameManager/UI/HUD_Hero.HUD_Hero_C|GetHUD (.AsHUD%20Hero (Utilities|Casting|CastToHUD_Hero (HUD|GetHUD (Game|GetPlayerController 0)))))) 0.0 1 "Forward" 1.0 false)
    (bind _asgm_game (Utilities|Casting|CastToGM_Game (Game|GetGameMode)))
    (Default|CheckWin _asgm_game)
    (Niagara|SpawnSystematLocation (Variables|Default|GetNiagara) (Transformation|GetActorLocation))
    (Actor|DestroyActor)))

(fn ConstructionScript)