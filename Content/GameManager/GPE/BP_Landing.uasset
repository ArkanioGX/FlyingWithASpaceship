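; BP_Landing is a landing spot actor that can spawn and hold a BP_Spaceship.
; On BeginPlay, if no valid ship is referenced and SpawnShip is set, it spawns one at the ShipPosition component's transform and stores it.
; GetSpaceShip returns the stored ship, creating it the same way on demand when missing, or returns nothing if spawning is disabled.
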(event EventBeginPlay
  (Utilities|IsValid (Variables|Default|GetSpaceShip)
    (:Is%20Not%20Valid
      (if (Variables|Default|GetspawnShip?)
        (bind _returnvalue (Game|SpawnActorfromClass "/Game/GameManager/Player/BP_Spaceship.BP_Spaceship_C" (Transformation|GetWorldTransform (Variables|Default|GetShipPosition)) "Undefined" "MultiplyWithRoot" 0 0))
        (Variables|Default|SetSpaceShip _returnvalue)))))

(fn ConstructionScript)

(fn GetSpaceShip
  (if (Utilities|IsValid (Variables|Default|GetSpaceShip))
    _
    (elif (Variables|Default|GetspawnShip?)
      (bind _returnvalue (Game|SpawnActorfromClass "/Game/GameManager/Player/BP_Spaceship.BP_Spaceship_C" (Transformation|GetWorldTransform (Variables|Default|GetShipPosition)) "Undefined" "MultiplyWithRoot" 0 0))
      (Variables|Default|SetSpaceShip _returnvalue)
      (else
        (return 0))))
  (return (Variables|Default|GetSpaceShip)))