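; BP_CollectableShip is a collectable pickup that awards score when the player touches it.
; On trigger overlap with the player pawn, it plays a 2D sound and adds a point through the PC_Hero controller's Score.
; It then asks GM_Base to check the win condition, spawns a Niagara effect at its location and destroys itself.
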(event OnComponentBeginOverlap(Trigger)
  (params (OverlappedComponent :type Primitive%20Component%20Object%20Reference) (OtherActor :type Actor%20Object%20Reference) (OtherComp :type Primitive%20Component%20Object%20Reference) (OtherBodyIndex :type Integer) (bFromSweep :type Boolean) (SweepResult :type Hit%20Result%20Structure%20%28by%20ref%29))
  ;[0 0 0 1 16] Check if it's player overlapping
  (if (== OtherActor (Game|Player|GetPlayerPawn 0))
    ;[0.0625 0 0 1 16] Play pickup sound
    (Audio|PlaySound2D (Variables|Default|GetSound) 1.0 1.0 0.0 0 0)
    (bind _aspc_hero (Utilities|Casting|CastToPC_Hero (Game|GetPlayerController 0)))
    (Default|AddScore (Variables|/Game/GameManager/Player/PC_Hero.PC_Hero_C|GetScore _aspc_hero) 1)
    ;[0.0625 0 0.0625 1 16] Check if player has won
    (Default|CheckWin (.AsGM%20Base (Utilities|Casting|CastToGM_Base (Game|GetGameMode))))
    ;[0 0.0625 0.0625 1 16] Spawn niagara instead of collectable
    (Niagara|SpawnSystematLocation (Variables|Default|GetNiagara) (Transformation|GetActorLocation))
    (Actor|DestroyActor)))

(fn ConstructionScript)