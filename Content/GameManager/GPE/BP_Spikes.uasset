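; BP_Spikes is a timed spike trap that cycles endlessly between retracted, warning and extended states.
; TurnOff, Warning and TurnOn chain through function-name timers from BeginPlay, each moving the Spikes component and playing a sound.
; Warning raises the spikes slightly as a harmless cue before full extension.
; TimeOff sets how long spikes stay extended, while TimeOn covers the retracted period including the warning.
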(event Custom|TurnOn
  ;[0 0 0 1 16] Turn on after some number of seconds
  (Utilities|Time|SetTimerbyFunctionName 0 "TurnOff" (Variables|Default|GetTimeOff))
  (Components|MoveComponentTo (Variables|Default|Getspikes) "0, 0, 0" "0.000000,0.000000,90.000000" false false 0.1 false)
  (Audio|PlaySoundatLocation "/Game/Assets/Audio/A_SpikeUnsheath.A_SpikeUnsheath" (Transformation|GetWorldLocation (Variables|Default|Getspikes)) "0, 0, 0" 1.0 1.0 0.0 0 0 0 0))

(event Custom|TurnOff
  ;[0 0.0625 0 1 16] Turn off after some number of seconds
  (Utilities|Time|SetTimerbyFunctionName 0 "Warning" (- (Variables|Default|GetTimeOn) (Variables|Default|GetWarningTime)))
  (Components|MoveComponentTo (Variables|Default|Getspikes) "0.000000,0.000000,-200.000000" "0.000000,0.000000,90.000000" false false 0.1 false)
  (Audio|PlaySoundatLocation "/Game/Assets/Audio/A_SpikeSheath.A_SpikeSheath" (Transformation|GetWorldLocation (Variables|Default|Getspikes)) "0, 0, 0" 1.0 1.0 0.0 0 0 0 0))

(event Custom|Warning
  ;[0.0625 0 0 1 16] Lift spikes barely, just to show them without causing any damage
  (Utilities|Time|SetTimerbyFunctionName 0 "TurnOn" (Variables|Default|GetWarningTime))
  (Components|MoveComponentTo (Variables|Default|Getspikes) "0.000000,0.000000,-160.000000" "0.000000,0.000000,90.000000" false false 0.06 false)
  (Audio|PlaySoundatLocation "/Game/Assets/Audio/A_SpikeWarning.A_SpikeWarning" (Transformation|GetWorldLocation (Variables|Default|Getspikes)) "0, 0, 0" 1.0 1.0 0.0 0 0 0 0))

(event EventBeginPlay
  (CallFunction|TurnOff))

(fn ConstructionScript)