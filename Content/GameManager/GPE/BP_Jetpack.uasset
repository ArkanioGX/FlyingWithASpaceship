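; BP_Jetpack is a one-time pickup that gives the player hero a jetpack or boosts the one they already have.
; On trigger overlap it assumes the player is responsible, casts player 0 to BP_Hero and plays a sound.
; An existing jetpack has its fuel capacity increased; otherwise a jetpack component is added, stored on the hero and attached to the mesh's Jetpack socket.
; Either path then destroys the pickup.
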(event OnComponentBeginOverlap(Trigger)
  (params (OverlappedComponent :type Primitive%20Component%20Object%20Reference) (OtherActor :type Actor%20Object%20Reference) (OtherComp :type Primitive%20Component%20Object%20Reference) (OtherBodyIndex :type Integer) (bFromSweep :type Boolean) (SweepResult :type Hit%20Result%20Structure%20%28by%20ref%29))
  (bind _asbp_hero (Utilities|Casting|CastToBP_Hero (Game|GetPlayerCharacter 0))) ; Assuming with player
  (Audio|PlaySound2D (Variables|Default|GetSound) 1.0 1.0 0.0 0 0) ; Playing audio effect
  (Utilities|IsValid (Variables|/Game/GameManager/Player/BP_Hero.BP_Hero_C|Getjetpack _asbp_hero) ; Was jetpack already picked up
    (:Is%20Valid
      (Default|IncreaseFuelCapacity (Variables|/Game/GameManager/Player/BP_Hero.BP_Hero_C|Getjetpack _asbp_hero)) ; Refueling
      (Actor|DestroyActor) ; Pickup is available only once
    )
    (:Is%20Not%20Valid
      (bind _returnvalue (AddComponent|AddBPJetpackSC :self _asbp_hero :RelativeTransform (Math|Transform|MakeTransform "0.000000,-60.000000,-25.000000" "0, 0, 0" "0.500000,0.500000,0.500000") :Character 0 :Fuel 3e+02 :FuelBar 0 :StartSound 0 :FlySound "/Game/Assets/Audio/JetPack/A_JetEngine_Loop.A_JetEngine_Loop" :Feedback 0 :LowFuelEffect 0 :LowFuelFeedback 0)) ; Adding jetpack feture to player
      (Variables|/Game/GameManager/Player/BP_Hero.BP_Hero_C|Setjetpack _asbp_hero _returnvalue) ; Saving it for future use
      (Transformation|AttachComponentToComponent _returnvalue (Variables|/Script/Engine.Character|GetMesh _asbp_hero) "Jetpack" "KeepRelative" "SnapToTarget" "KeepRelative" true) ; Attaching it to its socket
      (Components|StaticMesh|SetStaticMesh _returnvalue "/Game/Assets/Static_Mesh/SM_Barrel.SM_Barrel") ; Setting correct mesh
      (Actor|DestroyActor) ; Pickup is available only once
    )))

(fn ConstructionScript)