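; Actor component that lets the player board the spaceship, transferring control from the hero to the ship.
; On BeginPlay it caches the level's BP_Spaceship and BP_Hero.
; On IA_Transit, if the hero's capsule overlaps the ship's interaction sphere, it possesses the ship and swaps the Enhanced Input mapping context from default to spaceship.
; The hero is then hidden with capsule and mesh collision disabled, rather than destroyed.
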(event Input|EnhancedActionEvents|EnhancedInputActionIA_Transit
  (params (ActionValue :type Boolean) (ElapsedSeconds :type Float%20%28double-precision%29) (TriggeredSeconds :type Float%20%28double-precision%29) (InputAction :type Input%20Action%20Object%20Reference :default "/Game/GameManager/Player/Inputs/IA_Transit.IA_Transit"))
  (bind _returnvalue (Game|GetPlayerController 0))
  ;[0 0.0625 0 1 16] Check if able to enter into spaceship
  (if (Class|PrimitiveComponent|IsOverlappingComponent (Variables|/Game/GameManager/Player/BP_Spaceship.BP_Spaceship_C|GetHeroInteractionSphere (Variables|Default|GetSpaceship)) (Variables|/Script/Engine.Character|GetCapsuleComponent (Variables|Default|GetHero)))
    ;[0.0625 0.0625 0 1 16] Possess into spaceship
    (Pawn|UnPossess _returnvalue)
    (Pawn|Possess _returnvalue (Variables|Default|GetSpaceship))
    (Input|RemoveMappingContext (PlayerController|LocalPlayerSubsystems|GetEnhancedInputLocalPlayerSubsystem (Game|GetPlayerController 0)) "/Game/GameManager/Player/Inputs/IMC_Default.IMC_Default" "(bIgnoreAllPressedKeysUntilRelease=True,bForceImmediately=False,bNotifyUserSettings=False)")
    (Input|AddMappingContext (PlayerController|LocalPlayerSubsystems|GetEnhancedInputLocalPlayerSubsystem (Game|GetPlayerController 0)) "/Game/GameManager/Player/Inputs/IMC_Spaceship.IMC_Spaceship" 0 "(bIgnoreAllPressedKeysUntilRelease=True,bForceImmediately=False,bNotifyUserSettings=False)")
    ;[0 0 0.0625 1 16] Turn hero off
    (Rendering|SetActorHiddenInGame (Variables|Default|GetHero) true)
    (Collision|SetCollisionEnabled (Variables|/Script/Engine.Character|GetCapsuleComponent (Variables|Default|GetHero)) "NoCollision")
    (Collision|SetCollisionProfileName (Variables|/Script/Engine.Character|GetMesh (Variables|Default|GetHero)) "NoCollision" true :!class /Script/Engine.PrimitiveComponent)))

(event EventBeginPlay
  ;[0 0 0 1 16] Cache spaceship actor
  (bind _returnvalue (Actor|GetActorOfClass "/Game/GameManager/Player/BP_Spaceship.BP_Spaceship_C"))
  (Variables|Default|SetSpaceship _returnvalue)
  ;[0.0625 0 0 1 16] Cache hero actor
  (bind _returnvalue_2 (Actor|GetActorOfClass "/Game/GameManager/Player/BP_Hero.BP_Hero_C"))
  (Variables|Default|SetHero _returnvalue_2))