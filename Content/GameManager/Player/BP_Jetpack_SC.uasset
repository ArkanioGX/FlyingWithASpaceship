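; Jetpack scene component that lets BP_Hero fly while IA_Fly is held, spending fuel in flight and refilling on the ground.
; A downward trace measures height, and JetpackCurves shapes upward velocity below the height ceiling and pushes down above it.
; Tick updates fuel and the HUD fuel bar widget, while capacity upgrades reveal extra bars.
; Flight starts attached Niagara, sound and rumble feedback, and falling removes the effect.
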(event Custom|Start%20Effects
  ;[1 1 1] start feedback
  (Utilities|IsValid (Variables|Default|Getjetpack%20fire)
    (:Is%20Not%20Valid
      (bind _returnvalue (Niagara|SpawnSystemAttached (Variables|Default|GetEffect) (Variables|/Script/Engine.Character|GetMesh (Variables|Default|GetCharacter)) "Jetpack" "0.000000,-65.000000,0.000000" "-90.000000,0.000000,0.000000" "KeepRelativeOffset" false))
      (Variables|Default|Setjetpack%20fire _returnvalue)
      (Game|Feedback|ClientPlayForceFeedback (Game|GetPlayerController 0) (Variables|Default|GetFeedback) "None" false false false)
      (Audio|PlaySound2D (Variables|Default|GetStartSound) 1.0 1.0 0.0 0 0))))

(event Custom|End%20Effects
  ;[1 1 1] end feedback
  (Utilities|IsValid (Variables|Default|Getjetpack%20fire)
    (:Is%20Valid
      (Components|DestroyComponent (Variables|Default|Getjetpack%20fire)))))

(event Custom|Increase%20Fuel%20Capacity
  ;[1 1 1] upgrade fuel capacity
  (Variables|Default|SetMaxFuel (+ (Variables|Default|GetMaxFuel) (Variables|Default|GetFuelUnit)))
  (bind _result (Math|Integer|IncrementInt (Variables|Default|Getbar%20count))
    (:%20%20
      (Variables|/Script/UMG.Widget|SetVisibility (Utilities|Array|Get(acopy) (Variables|Default|GetA_ProgressBars) _result) "Visible"))))

(event Custom|set%20up%20Fuel%20UI
  (bind _fuelbar (Variables|Default|GetFuelBar))
  ;[1 1 1] make and populate array of fuel bars
  (bind _output_get (Variables|Default|SetA_ProgressBars (Utilities|Array|MakeArray (Variables|/Game/GameManager/UI/W_FuelBar.W_FuelBar_C|GetProgressBar _fuelbar))))
  (Utilities|Array|Add _output_get (Variables|/Game/GameManager/UI/W_FuelBar.W_FuelBar_C|GetProgressBar_1 _fuelbar))
  (Utilities|Array|Add _output_get (Variables|/Game/GameManager/UI/W_FuelBar.W_FuelBar_C|GetProgressBar_2 _fuelbar))
  (Utilities|Array|Add _output_get (Variables|/Game/GameManager/UI/W_FuelBar.W_FuelBar_C|GetProgressBar_3 _fuelbar))
  (Utilities|Array|Add _output_get (Variables|/Game/GameManager/UI/W_FuelBar.W_FuelBar_C|GetProgressBar_4 _fuelbar))
  (for _array_element (Variables|Default|GetA_ProgressBars)
    (Variables|/Script/UMG.Widget|SetVisibility _array_element "Hidden"))
  (Variables|/Script/UMG.Widget|SetVisibility (Utilities|Array|Get(acopy) (Variables|Default|GetA_ProgressBars)) "Visible"))

(event Input|EnhancedActionEvents|EnhancedInputActionIA_Fly
  (params (ActionValue :type Float%20%28double-precision%29) (ElapsedSeconds :type Float%20%28double-precision%29) (TriggeredSeconds :type Float%20%28double-precision%29) (InputAction :type Input%20Action%20Object%20Reference :default "/Game/GameManager/Player/Inputs/IA_Fly.IA_Fly"))
  (bind _jetpackcurves (Variables|Default|GetJetpackCurves))
  (bind _jetpackcurves_2 (Variables|Default|GetJetpackCurves))
  (bind _character (Variables|Default|GetCharacter))
  (bind _character_2 (Variables|Default|GetCharacter))
  (bind _returnvalue (Transformation|GetVelocity _character))
  (bind _returnvalue_2 (Transformation|GetVelocity _character_2))
  (:Triggered
    (if (not (and (AI|Components|NavMovement|IsMovingonGround (Variables|/Script/Engine.Character|GetCharacterMovement (Variables|Default|GetCharacter))) (< (Variables|Default|GetFuel) (Variables|Default|GetFuel%20Threshold))))
      (if (>= (Variables|Default|GetFuel) 0.0)
        (Pawn|Components|CharacterMovement|SetMovementMode (Variables|/Script/Engine.Character|GetCharacterMovement (Variables|Default|GetCharacter)) "MOVE_Flying" 0)
        ;[1 1 1] Check player height off the ground
        (CallFunction|StartEffects)
        (bind _outhit (Collision|LineTraceByChannel (Transformation|GetWorldLocation) (+ (Transformation|GetWorldLocation) (Math|Vector|MakeVector 0.0 0.0 -1e+05)) "TraceTypeQuery1" false 0 "None"))
        (if (<= (/ (.distance _outhit) (.maxheight (Variables|Default|GetJetpackCurves))) 1.0)
          ;[1 1 1] Float upwards
          (Variables|/Script/Engine.MovementComponent|SetVelocity (Variables|/Script/Engine.Character|GetCharacterMovement (Variables|Default|GetCharacter)) (Math|Vector|MakeVector (.x _returnvalue_2) (.y _returnvalue_2) (* (Math|Curves|GetFloatValue (.actuationcurve _jetpackcurves_2) ActionValue) (* (.maxforce _jetpackcurves_2) (Math|Curves|GetFloatValue (.upwardcurve _jetpackcurves_2) (/ (.distance _outhit) (.maxheight _jetpackcurves_2)))))))
          (else
            ;[1 1 1] Lerp down
            (Variables|/Script/Engine.MovementComponent|SetVelocity (Variables|/Script/Engine.Character|GetCharacterMovement (Variables|Default|GetCharacter)) (Math|Vector|MakeVector (.x _returnvalue) (.y _returnvalue) (* (* (Math|Float|Clamp(Float) (- (.distance _outhit) (.maxheight _jetpackcurves)) 0.0 (.maxheight _jetpackcurves)) (.downwardlerp _jetpackcurves)) -1.0)))))
        (else
          ;[1 1 1] Start falling again
          (Pawn|Components|CharacterMovement|SetMovementMode (Variables|/Script/Engine.Character|GetCharacterMovement (Variables|Default|GetCharacter)) "MOVE_Falling" 0 :!label _label)
          (CallFunction|EndEffects)))))
  (:Completed
    (goto _label)))

(event EventTick
  (params (DeltaSeconds :type Float%20%28single-precision%29))
  (bind _character (Variables|Default|GetCharacter))
  (bind _charactermovement (Variables|/Script/Engine.Character|GetCharacterMovement _character))
  ;[1 1 1] update fuel count
  (if (and (AI|Components|NavMovement|IsMovingonGround _charactermovement) (< (Variables|Default|GetFuel) (Variables|Default|GetMaxFuel)))
    ;;[1 1 1] if on ground and fuel isnt max, increment fuel
    (Variables|Default|SetFuel (+ (Variables|Default|GetFuel) (.refuelspeed (Variables|Default|GetJetpackCurves))))
    (Variables|/Game/GameManager/UI/W_FuelBar.W_FuelBar_C|Setfuel (Variables|Default|GetFuelBar) (Variables|Default|GetFuel) :!label _label)
    (else
      ;;[1 1 1] if flying, decrement fuel
      (if (Class|NavMovementComponent|IsFlying _charactermovement)
        (Math|Float|DecrementFloat (Variables|Default|GetFuel)
          (:%20%20
            (goto _label)))))))

(event EventBeginPlay
  ;[1 1 1] create fuel bar widget
  (Variables|Default|SetFuelUnit (.maxfuel (Variables|Default|GetJetpackCurves)))
  (Variables|Default|SetMaxFuel (Variables|Default|GetFuelUnit))
  (Variables|Default|SetFuel (Variables|Default|GetMaxFuel))
  (bind _returnvalue (UserInterface|CreateWidget "/Game/GameManager/UI/W_FuelBar.W_FuelBar_C" (Game|GetPlayerController 0)))
  (bind _output_get (Variables|Default|SetFuelBar _returnvalue))
  (CallFunction|SetUpFuelUI)
  (UserInterface|Viewport|AddtoViewport _output_get 0)
  (bind _asbp_hero (Utilities|Casting|CastToBP_Hero (Game|GetPlayerCharacter 0)))
  (Variables|Default|SetCharacter _asbp_hero)
  (Variables|/Game/GameManager/UI/W_FuelBar.W_FuelBar_C|Setfuel (Variables|Default|GetFuelBar) (Variables|Default|GetFuel))
  (Variables|/Game/GameManager/UI/W_FuelBar.W_FuelBar_C|SetfuelUnit (Variables|Default|GetFuelBar) (Variables|Default|GetFuelUnit)))