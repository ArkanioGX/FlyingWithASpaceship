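; Actor component on BP_Spaceship that handles the player's exit from the ship into the hero at landing zones.
; On IA_Transit while overlapping a BP_Landing, it possesses BP_Hero, plays that zone's music, swaps input mapping contexts and restores ship gravity.
; It then moves both actors to the zone's markers and re-enables hero visibility and collision.
; While the ship is piloted, Tick pins the hero to its location to avoid interpolation on exit.
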(event Input|EnhancedActionEvents|EnhancedInputActionIA_Transit
  (params (ActionValue :type Boolean) (ElapsedSeconds :type Float%20%28double-precision%29) (TriggeredSeconds :type Float%20%28double-precision%29) (InputAction :type Input%20Action%20Object%20Reference :default "/Game/GameManager/Player/Inputs/IA_Transit.IA_Transit"))
  (bind _hero (Variables|Default|GetHero))
  (bind _currentspaceship (Variables|Default|GetCurrentSpaceship))
  (bind _capsulecomponent (Variables|/Script/Engine.Character|GetCapsuleComponent _currentspaceship))
  (bind _overlappingactors (Collision|GetOverlappingActors _capsulecomponent "/Game/GameManager/GPE/BP_Landing.BP_Landing_C" :!class /Script/Engine.PrimitiveComponent))
  (bind _output (Utilities|Array|Get(acopy) _overlappingactors))
  (bind _asbp_landing (Utilities|Casting|CastToBP_Landing _output))
  ;[0 0.0625 0 1 16] Check if able to exit from spaceship
  (if (Utilities|Array|IsNotEmpty _overlappingactors)
    ;[0.0625 0.0625 0 1 16] Possess into hero
    (Pawn|Possess (Game|GetPlayerController 0) _hero)
    (Default|PlayMusic _hero (Variables|/Game/GameManager/GPE/BP_Landing.BP_Landing_C|GetMusic (.AsBP%20Landing (Utilities|Casting|CastToBP_Landing _output))))
    (Input|RemoveMappingContext (PlayerController|LocalPlayerSubsystems|GetEnhancedInputLocalPlayerSubsystem (Game|GetPlayerController 0)) "/Game/GameManager/Player/Inputs/IMC_Spaceship.IMC_Spaceship" "(bIgnoreAllPressedKeysUntilRelease=True,bForceImmediately=False,bNotifyUserSettings=False)")
    (Input|AddMappingContext (PlayerController|LocalPlayerSubsystems|GetEnhancedInputLocalPlayerSubsystem (Game|GetPlayerController 0)) "/Game/GameManager/Player/Inputs/IMC_Default.IMC_Default" 0 "(bIgnoreAllPressedKeysUntilRelease=True,bForceImmediately=False,bNotifyUserSettings=False)")
    (Variables|/Script/Engine.CharacterMovementComponent|SetGravityScale (Variables|/Script/Engine.Character|GetCharacterMovement (Variables|Default|GetCurrentSpaceship)) 1.0)
    ;[0.0625 0 0.0625 1 16] Teleport hero and Spaceship when leaving spaceship
    (Transformation|SetActorLocation (Variables|Default|GetCurrentSpaceship) (Transformation|GetWorldLocation (Variables|/Game/GameManager/GPE/BP_Landing.BP_Landing_C|GetShipPosition _asbp_landing)) false false)
    (Transformation|SetActorLocation (Variables|Default|GetHero) (Transformation|GetWorldLocation (Variables|/Game/GameManager/GPE/BP_Landing.BP_Landing_C|GetPlayerPosition _asbp_landing)) false false)
    ;[0 0 0.0625 1 16] Turn hero on
    (Rendering|SetActorHiddenInGame (Variables|Default|GetHero) false)
    (Collision|SetCollisionEnabled (Variables|/Script/Engine.Character|GetCapsuleComponent (Variables|Default|GetHero)) "QueryAndPhysics")
    (Collision|SetCollisionProfileName (Variables|/Script/Engine.Character|GetMesh (Variables|Default|GetHero)) "CharacterMesh" true :!class /Script/Engine.PrimitiveComponent)))

(event EventBeginPlay
  ;[0 0 0 1 16] Cache hero actor
  (bind _returnvalue (Actor|GetActorOfClass "/Game/GameManager/Player/BP_Hero.BP_Hero_C"))
  (Variables|Default|SetHero _returnvalue)
  ;[0.0625 0 0 1 16] Cache spaceship actor
  (bind _asbp_spaceship (Utilities|Casting|CastToBP_Spaceship (Components|GetOwner)))
  (Variables|Default|SetCurrentSpaceship _asbp_spaceship)
  ;[1 1 1] Cache Landing Zones
  (bind _outactors (Actor|GetAllActorsOfClass "/Game/GameManager/GPE/BP_Landing.BP_Landing_C"))
  (Variables|Default|SetLandingZones _outactors))

(event EventTick
  (params (DeltaSeconds :type Float%20%28single-precision%29))
  ;[0.0625 0 0.0625 1 16] Teleport hero to avoid interpolation
  (Utilities|Casting|CastToBP_Spaceship (Game|Player|GetPlayerPawn 0))
  (Transformation|SetActorLocation (Variables|Default|GetHero) (+ (Transformation|GetActorLocation (Variables|Default|GetCurrentSpaceship)) (* (Transformation|GetActorForwardVector (Variables|Default|GetCurrentSpaceship)) "")) false false))