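; BP_Score_AC is a player score component that accumulates points through a single AddScore function.
; Each addition makes every BP_CoinDoor actor in the level run CheckScore.
; It then reaches the HUD widget through the first player controller's HUD_Hero, pushes the truncated score to it, plays a widget animation and returns the new total.
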(fn AddScore
  (params (Add%20score :type Integer))
  (bind _returnvalue (Game|GetPlayerController 0))
  (bind _returnvalue_2 (HUD|GetHUD _returnvalue))
  (bind _ashud_hero (Utilities|Casting|CastToHUD_Hero _returnvalue_2))
  (bind _hud (Variables|/Game/GameManager/UI/HUD_Hero.HUD_Hero_C|GetHUD _ashud_hero))
  (bind _output_get (Variables|Default|SetScore (+ Add%20score (Variables|Default|GetScore))))
  (bind _outactors (Actor|GetAllActorsOfClass "/Game/GameManager/GPE/BP_CoinDoor.BP_CoinDoor_C"))
  (for _array_element _outactors
    (Default|CheckScore _array_element))
  (Default|ScoreUpdate (Variables|/Game/GameManager/UI/HUD_Hero.HUD_Hero_C|GetHUD (.AsHUD%20Hero (Utilities|Casting|CastToHUD_Hero (HUD|GetHUD (Game|GetPlayerController 0))))) (Math|Float|Truncate (Math|Conversions|ToFloat(Integer) (Math|Float|Truncate _output_get))))
  (UserInterface|Animation|PlayAnimation _hud (Variables|/Game/GameManager/UI/W_GameUI.W_GameUI_C|GetNewAnimation _hud) 0.0 1 "Forward" 1.0 false)
  (return (Math|Float|Truncate _output_get)))