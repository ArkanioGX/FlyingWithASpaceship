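; Player controller that sets up input and relays player-level calls to the pawn and game mode.
; On BeginPlay it adds the hero or spaceship Enhanced Input mapping context based on whether the pawn is a BP_Hero, then switches to game-only input.
; Respawn goes through the BP_Player cast, hiding pawn differences from callers, and clears IsDead.
; CheckWin forwards to GM_Base.
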(event Custom|Respawn
  ;[0.0625 0 0 1 16] Abstract player's bluprint difference passing all player calls here and distribute them around
  (Default|Respawn (.AsBP%20Player (Utilities|Casting|CastToBP_Player (Game|Player|GetPlayerPawn 0))))
  (Variables|Default|SetIsDead false))

(event Custom|CheckWin
  ;[0.0625 0 0 1 16] Abstract player's bluprint difference passing all player calls here and distribute them around
  (Default|CheckWin (.AsGM%20Base (Utilities|Casting|CastToGM_Base (Game|GetGameMode)))))

(event EventBeginPlay
  ;[0 0 0 1 16] Select hero or spaceship input mapping context depending on player's blueprint at startup
  (Input|AddMappingContext (PlayerController|LocalPlayerSubsystems|GetEnhancedInputLocalPlayerSubsystem) (select (.bSuccess (Utilities|Casting|CastToBP_Hero (Game|Player|GetPlayerPawn 0))) "/Game/GameManager/Player/Inputs/IMC_Default.IMC_Default" "/Game/GameManager/Player/Inputs/IMC_Spaceship.IMC_Spaceship") 0 "(bIgnoreAllPressedKeysUntilRelease=True,bForceImmediately=False,bNotifyUserSettings=False)")
  (Input|SetInputModeGameOnly self false))

(fn ConstructionScript)