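; Player jetpack component that flies the third-person character while IA_Fly is held and fuel remains, with sound, force feedback and Niagara effects.
; A downward trace measures height, so JetpackCurves can shape upward velocity by input and altitude, or push the player down above max height.
; Releasing input or running out of fuel restores Falling.
; Tick refills fuel on the ground, drains it in flight and updates the fuel bar widget.
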(event Input|EnhancedActionEvents|EnhancedInputActionIA_Fly
  (params (ActionValue :type Float%20%28double-precision%29) (ElapsedSeconds :type Float%20%28double-precision%29) (TriggeredSeconds :type Float%20%28double-precision%29) (InputAction :type Input%20Action%20Object%20Reference :default "/Game/Player/Jetpack/InputActions/IA_Fly.IA_Fly"))
  (bind _jetpackcurves (Variables|Default|GetJetpackCurves))
  (bind _jetpackcurves_2 (Variables|Default|GetJetpackCurves))
  (bind _character (Variables|Default|GetCharacter))
  (bind _character_2 (Variables|Default|GetCharacter))
  (bind _returnvalue (Transformation|GetVelocity _character))
  (bind _returnvalue_2 (Transformation|GetVelocity _character_2))
  (:Triggered
    (if (Utilities|Enum|Equal(Enum) (Variables|/Script/Engine.CharacterMovementComponent|GetMovementMode (Variables|/Script/Engine.Character|GetCharacterMovement (Variables|Default|GetCharacter))) "MOVE_Walking")
      (Audio|PlaySound2D (Variables|Default|GetStartSound) 1.0 1.0 0.0 0 0))
    (ForceFeedback|SpawnForceFeedbackAttached (Variables|Default|GetFeedback) self "None" "0, 0, 0" "0, 0, 0" "KeepRelativeOffset" false false 1.0 0.0 0)
    (if (>= (Variables|Default|GetFuel) 0.0)
      (Pawn|Components|CharacterMovement|SetMovementMode (Variables|/Script/Engine.Character|GetCharacterMovement (Variables|Default|GetCharacter)) "MOVE_Flying" 0)
      ;[1 1 1] Check player height off the ground
      (bind _outhit (Collision|LineTraceByChannel (Transformation|GetWorldLocation) (+ (Transformation|GetWorldLocation) (Math|Vector|MakeVector 0.0 0.0 -1e+05)) "TraceTypeQuery1" false 0 "None"))
      (if (<= (/ (.distance _outhit) (.maxheight (Variables|Default|GetJetpackCurves))) 1.0)
        ;[1 1 1] Float upwards
        (Variables|/Script/Engine.MovementComponent|SetVelocity (Variables|/Script/Engine.Character|GetCharacterMovement (Variables|Default|GetCharacter)) (Math|Vector|MakeVector (.x _returnvalue_2) (.y _returnvalue_2) (* (Math|Curves|GetFloatValue (.actuationcurve _jetpackcurves_2) ActionValue) (* (.maxforce _jetpackcurves_2) (Math|Curves|GetFloatValue (.upwardcurve _jetpackcurves_2) (/ (.distance _outhit) (.maxheight _jetpackcurves_2)))))))
        (Audio|PlaySound2D (Variables|Default|GetFlySound) 1.0 1.0 0.0 0 0)
        (Niagara|SpawnSystemAttached (Variables|Default|GetEffect) self "Effect" "0, 0, 0" "0, 0, 0" "KeepRelativeOffset" true)
        (else
          ;[1 1 1] Lerp down
          (Variables|/Script/Engine.MovementComponent|SetVelocity (Variables|/Script/Engine.Character|GetCharacterMovement (Variables|Default|GetCharacter)) (Math|Vector|MakeVector (.x _returnvalue) (.y _returnvalue) (* (* (Math|Float|Clamp(Float) (- (.distance _outhit) (.maxheight _jetpackcurves)) 0.0 (.maxheight _jetpackcurves)) (.downwardlerp _jetpackcurves)) -1.0)))))
      (else
        ;[1 1 1] Start falling again
        (Pawn|Components|CharacterMovement|SetMovementMode (Variables|/Script/Engine.Character|GetCharacterMovement (Variables|Default|GetCharacter)) "MOVE_Falling" 0 :!label _label))))
  (:Completed
    (goto _label)))

(event EventTick
  (params (DeltaSeconds :type Float%20%28single-precision%29))
  (bind _character (Variables|Default|GetCharacter))
  (bind _jetpackcurves (Variables|Default|GetJetpackCurves))
  (bind _charactermovement (Variables|/Script/Engine.Character|GetCharacterMovement _character))
  ;[1 1 1] update fuel count
  (if (and (AI|Components|NavMovement|IsMovingonGround _charactermovement) (< (Variables|Default|GetFuel) (.maxfuel _jetpackcurves)))
    ;;[1 1 1] if on ground and fuel isnt max, increment fuel
    (Math|Float|IncrementFloat (Variables|Default|GetFuel)
      (:%20%20
        (Variables|/Game/Player/ThirdPerson/Blueprints/W_FuelBar.W_FuelBar_C|Setpercentage (Variables|Default|GetFuelBar) (/ (Variables|Default|GetFuel) (.maxfuel _jetpackcurves)) :!label _label)))
    (else
      ;;[1 1 1] if flying, decrement fuel
      (if (Class|NavMovementComponent|IsFlying _charactermovement)
        (Math|Float|DecrementFloat (Variables|Default|GetFuel)
          (:%20%20
            (goto _label)))))))

(event EventBeginPlay
  (Variables|Default|SetFuel (Variables|Default|GetMaxFuel))
  (bind _returnvalue (UserInterface|CreateWidget "/Game/Player/ThirdPerson/Blueprints/W_FuelBar.W_FuelBar_C"))
  (bind _output_get (Variables|Default|SetFuelBar _returnvalue))
  (UserInterface|Viewport|AddtoViewport _returnvalue 0)
  (bind _asbp_third_person_character (Utilities|Casting|CastToBP_ThirdPersonCharacter (Game|GetPlayerCharacter 0)))
  (Variables|Default|SetCharacter _asbp_third_person_character))